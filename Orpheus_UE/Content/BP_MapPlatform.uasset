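; BP_MapPlatform is a map platform actor that builds a segmented strip with a three-lane grid of positions on top.
; Its construction script tiles meshes along local X to fit the End vector's length, using the base mesh's bounds.
; Each segment gets ten columns of three scaled meshes, whose local positions fill Points.
; GetPosition maps Row and Col into Points, adding only actor location, so rotation is ignored.
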(fn `GetPosition`
  (params (row :type Byte) (col :type Byte))
  (returns (ReturnValue :type "Vector Structure"))
  (return (+ (`|GetArrayItem` (`self.Points`) (`KismetMathLibrary.Conv_ByteToInt` (+ row (* col 3)))) (`self.K2_GetActorLocation`))))

(fn `UserConstructionScript`
  (locals (TempLoc :type "Vector Structure"))
  (bind (_origin _boxextent) (`KismetSystemLibrary.GetComponentBounds` (`self.StaticMeshComponent`)))
  (bind (_origin_2 _boxextent_2) (`KismetSystemLibrary.GetComponentBounds` (`self.StaticMeshComponent`)))
  (bind _returnvalue (/ (.x _boxextent) 5.0))
  (bind _returnvalue_2 (/ (* (.y _boxextent) 2.0) 3.0))
  (bind _returnvalue_3 (`KismetMathLibrary.FTrunc` (/ (- (`KismetMathLibrary.VSize` (`self.End`)) (.x _boxextent_2)) (* (.x _boxextent_2) 2.0))))
  (bind _returnvalue_4 (/ _returnvalue_2 2.0))
  (`KismetArrayLibrary.Array_Clear` (`self.Points`))
  (for _index (range 1 (+ _returnvalue_3 1))
    (`AddComponent|NODE_AddStaticMeshComponent-3` :`RelativeTransform` (`KismetMathLibrary.MakeTransform` (`KismetMathLibrary.MakeVector` (* (.x _boxextent_2) 2.0 _index)))))
  (set `local.TempLoc` (`KismetMathLibrary.MakeVector` (* (.x _boxextent) -1.0) (* (.y _boxextent) -1.0) (.z _boxextent)))
  (for _ (range (+ _returnvalue_3 1))
    (for _index_2 (range 1 11)
      (bind _returnvalue_5 (- (+ (`local.TempLoc`) (`KismetMathLibrary.MakeVector` (* _returnvalue _index_2) 0.0 26.0)) (`KismetMathLibrary.MakeVector` (/ _returnvalue 2.0))))
      (bind _returnvalue_6 (+ _returnvalue_5 (`KismetMathLibrary.MakeVector` 0.0 _returnvalue_4)))
      (`KismetArrayLibrary.Array_Add` (`self.Points`) _returnvalue_6)
      (`AddComponent|NODE_AddStaticMeshComponent-6` :`RelativeTransform` (`KismetMathLibrary.MakeTransform` _returnvalue_6 (struct) (1.5 0.6 1.0)))
      (bind _returnvalue_7 (- (+ _returnvalue_5 (`KismetMathLibrary.MakeVector` 0.0 (* _returnvalue_2 2.0))) (`KismetMathLibrary.MakeVector` 0.0 _returnvalue_4)))
      (`KismetArrayLibrary.Array_Add` (`self.Points`) _returnvalue_7)
      (`AddComponent|NODE_AddStaticMeshComponent-7` :`RelativeTransform` (`KismetMathLibrary.MakeTransform` _returnvalue_7 (struct) (1.5 0.6 1.0)))
      (bind _returnvalue_8 (- (+ _returnvalue_5 (`KismetMathLibrary.MakeVector` 0.0 (* _returnvalue_2 3.0))) (`KismetMathLibrary.MakeVector` 0.0 _returnvalue_4)))
      (`KismetArrayLibrary.Array_Add` (`self.Points`) _returnvalue_8)
      (`AddComponent|NODE_AddStaticMeshComponent-9` :`RelativeTransform` (`KismetMathLibrary.MakeTransform` _returnvalue_8 (struct) (1.5 0.6 1.0))))
    (set `local.TempLoc` (+ (`local.TempLoc`) (`KismetMathLibrary.MakeVector` (* (.x _boxextent) 2.0))))))